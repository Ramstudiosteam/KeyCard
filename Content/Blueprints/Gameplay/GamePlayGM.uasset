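; Gameplay game mode that tracks player controllers, respawns players as their selected character and handles logout.
; Controllers received through OnSwapPlayerControllers are added to AllPlayerControllers.
; RespawnPlayer destroys the current pawn, spawns the given character class using randomly picked PlayerStart transforms, then possesses it.
; On logout, an exiting GamePlayPC is passed to GameInfoInstance's DestroySessionCaller to tear down its session.
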(event `self.K2_OnSwapPlayerControllers`
  (params (OldPC :type "PlayerController Object Reference") (NewPC :type "PlayerController Object Reference"))
  ;[1 1 1] Keeps track of connected players
  (`KismetArrayLibrary.Array_Add` (`self.AllPlayerControllers`) NewPC))

(event `RespawnPlayer`
  (params (`Player Controller` :type "PlayerController Object Reference") (`Player Character` :type "Character Class Reference"))
  (bind _returnvalue (`Controller.K2_GetPawn` `Player Controller`))
  (bind _spawnpoints (`self.SpawnPoints`))
  (bind (_returnvalue_location _returnvalue_rotation) (`KismetMathLibrary.BreakTransform` (`self.GetTransform` (`|GetArrayItem` _spawnpoints (`KismetMathLibrary.RandomIntegerInRange` 0 (- (`KismetArrayLibrary.Array_Length` _spawnpoints) 1))))))
  ;[1 1 1] Spawn The Player With Thier Selected Character
  (bind _outactors (`GameplayStatics.GetAllActorsOfClass` "/Script/Engine.PlayerStart"))
  (set `self.SpawnPoints` _outactors)
  (`/Engine/EditorBlueprintResources/StandardMacros.IsValid` _returnvalue
    (:`Is Valid`
      (`self.K2_DestroyActor` _returnvalue))
    (:`Is Not Valid`
      _))
  (bind _returnvalue_2 (`|SpawnActorFromClass` `Player Character` (`KismetMathLibrary.MakeTransform` _returnvalue_location _returnvalue_rotation) "Undefined" "OverrideRootScale"))
  (`Controller.Possess` `Player Controller` _returnvalue_2))

(event `self.K2_OnLogout`
  (params (ExitingController :type "Controller Object Reference"))
  ;[1 1 1] Destroy Session When Logout
  (bind _asgame_play_pc (cast `/Game/Blueprints/Gameplay/GamePlayPC` ExitingController))
  (`/Game/Blueprints/AllLevels/GameInfoInstance.DestroySessionCaller` (cast `/Game/Blueprints/AllLevels/GameInfoInstance` (`GameplayStatics.GetGameInstance`) :!pure true) _asgame_play_pc))

(fn `UserConstructionScript`)