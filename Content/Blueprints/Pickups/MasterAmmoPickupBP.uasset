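; Base ammo pickup actor that responds when a 0_Base character enters or leaves its sphere trigger.
; On overlap begin it stores the character, turns on the mesh's custom depth rendering and passes itself to the character's EnableInputs.
; On overlap end it turns custom depth off, with no matching call to disable inputs.
; The file itself contains no ammo-granting logic.
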(event `self.Sphere.OnComponentBeginOverlap`
  (params (OverlappedComponent :type "PrimitiveComponent Object Reference") (OtherActor :type "Actor Object Reference") (OtherComp :type "PrimitiveComponent Object Reference") (OtherBodyIndex :type Integer) (bFromSweep :type Boolean) (SweepResult :type "HitResult Structure (by ref)"))
  (bind _as0_base (cast `/Game/Blueprints/Characters/0_Base` OtherActor))
  (set `self.PlayerCharacter` _as0_base)
  (`PrimitiveComponent.SetRenderCustomDepth` (`self.StaticMesh`) true)
  (`/Game/Blueprints/Characters/0_Base.EnableInputs` (`self.PlayerCharacter`) self))

(event `self.Sphere.OnComponentEndOverlap`
  (params (OverlappedComponent :type "PrimitiveComponent Object Reference") (OtherActor :type "Actor Object Reference") (OtherComp :type "PrimitiveComponent Object Reference") (OtherBodyIndex :type Integer))
  (bind _as0_base (cast `/Game/Blueprints/Characters/0_Base` OtherActor))
  (set `self.PlayerCharacter` _as0_base)
  (`PrimitiveComponent.SetRenderCustomDepth` (`self.StaticMesh`) false))

(fn `UserConstructionScript`)