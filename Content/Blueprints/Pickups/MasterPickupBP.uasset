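; Base weapon pickup Blueprint that stores the overlapping 0_Base character, hides its prompt and outline, and handles firing and reloading.
; Firing loops through a delayed Gate, using line traces for interface-based damage and spawning projectiles aimed at the trace result.
; Ammo lives in ItemInfo, refilled from reserve by manual reload or on trigger release when empty.
; Pickup input and prompt-showing chains are partly unwired; overlap destroys the trigger sphere immediately.
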(event `self.Sphere.OnComponentBeginOverlap`
  (params (OverlappedComponent :type "PrimitiveComponent Object Reference") (OtherActor :type "Actor Object Reference") (OtherComp :type "PrimitiveComponent Object Reference") (OtherBodyIndex :type Integer) (bFromSweep :type Boolean) (SweepResult :type "HitResult Structure (by ref)"))
  ;[1 1 1] Begin / End Overlap
  (bind _as0_base (cast `/Game/Blueprints/Characters/0_Base` OtherActor))
  (set `self.PlayerCharacter` _as0_base)
  (`self.OffAll`))

(event `self.Sphere.OnComponentEndOverlap`
  (params (OverlappedComponent :type "PrimitiveComponent Object Reference") (OtherActor :type "Actor Object Reference") (OtherComp :type "PrimitiveComponent Object Reference") (OtherBodyIndex :type Integer))
  ;[1 1 1] Begin / End Overlap
  (bind _as0_base (cast `/Game/Blueprints/Characters/0_Base` OtherActor))
  (set `self.PlayerCharacter` _as0_base))

(event `PickServerInput`
  ;[1 1 1] Get Input
  (if (`self.CanWePick?`) :!label _label
    (`/Game/Blueprints/Characters/0_Base.Pickup` (`self.PlayerCharacter`) self)))

(event `PickClientInput`
  ;[1 1 1] Get Input
  (goto _label))

(event `InputAction|ItemInteraction`
  (params (Key :type "Key Structure" :default "AnyKey"))
  ;[1 1 1] Get Input
)

(event `OffAll`
  (bind _sphere (`self.Sphere`))
  ;[1 1 1] Off Components
  (`self.On/OffVisibility/CustomDepth` false)
  (`/Engine/EditorBlueprintResources/StandardMacros.IsValid` _sphere
    (:`Is Valid`
      (`ActorComponent.K2_DestroyComponent` _sphere))))

(event `StartFire`
  (params (Start :type "Vector Structure") (End :type "Vector Structure") (Location :type "Vector Structure"))
  (bind _returnvalue (`SceneComponent.GetSocketLocation` (`self.SkeletalMesh`) "Muzzle"))
  ;[1 1 1] Fire Weapon System
  (`|ExecutionSequence`
    (:`then_0`
      (goto _label_2 :!via `Open`))
    (:`then_1`
      (`/Engine/EditorBlueprintResources/StandardMacros.Gate` true :!label _label_2
        (:`Exit`
          (`|ExecutionSequence`
            (:`then_0`
              (`KismetSystemLibrary.RetriggerableDelay` 0.2)
              (goto _label_2))
            (:`then_1`
              (if (<= (`.CurrentAmmo_10_F26B1AC041A51A8482A4EC9820B606C3` (break `/Game/Blueprints/Pickups/ItemType` (`self.ItemInfo`))) 0)
                (`KismetSystemLibrary.PrintString` "Out Of AMMO")
                (else
                  (`SkeletalMeshComponent.PlayAnimation` (`self.SkeletalMesh`) "/Game/Blueprints/Pickups/Weapons/SciFiWeapLight/Weapons/Anims/Fire_Rifle_W.Fire_Rifle_W" false)
                  (`Character.PlayAnimMontage` (`self.PlayerCharacter`) "/Game/Animations/RifleAnimsetPro/Animations/InPlace/Rifle_ShootOnce_Montage.Rifle_ShootOnce_Montage" 1.0 "None")
                  (`GameplayStatics.PlaySoundAtLocation` "/Game/StarterContent/Audio/Explosion_Cue.Explosion_Cue" Location)
                  (bind (_outhit _returnvalue_2) (`KismetSystemLibrary.LineTraceSingle` :`Start` Start :`End` End :`TraceChannel` "TraceTypeQuery3" :`DrawDebugType` "ForOneFrame"))
                  (if _returnvalue_2
                    _
                    (else
                      _))
                  (setmembers `/Game/Blueprints/Pickups/ItemType` :`StructRef` (`self.ItemInfo`) :`CurrentAmmo` (- (`.CurrentAmmo_10_F26B1AC041A51A8482A4EC9820B606C3` (break `/Game/Blueprints/Pickups/ItemType` (`self.ItemInfo`))) 1))
                  (bind (_bblockinghit _binitialoverlap _time _location _impactpoint _normal _impactnormal _physmat _hitactor _hitcomponent _hitbonename _hititem _faceindex _tracestart _traceend) (`GameplayStatics.BreakHitResult` _outhit))
                  (if (`KismetSystemLibrary.DoesImplementInterface` _hitactor "/Game/Blueprints/Interfaces/TakeDamage.TakeDamage_C")
                    (message `/Game/Blueprints/Interfaces/TakeDamage.iTakeDamage` _hitactor _hitbonename (`KismetMathLibrary.RandomFloatInRange` 15.0 15.0) (`self.PlayerCharacter`)))
                  (`|SpawnActorFromClass` "/Game/Blueprints/Pickups/Weapons/Projectiles/BaseProjectileBP.BaseProjectileBP_C" (`KismetMathLibrary.MakeTransform` _returnvalue (`KismetMathLibrary.FindLookAtRotation` _returnvalue (`KismetMathLibrary.SelectVector` _impactpoint _traceend _returnvalue_2))) "Undefined" "OverrideRootScale")
                  (`GameplayStatics.SpawnEmitterAtLocation` "/Game/Blueprints/Pickups/Weapons/SciFiWeapLight/FX/Particles/P_Impact_Metal_Medium_Dark.P_Impact_Metal_Medium_Dark" _location))))))))))

(event `StopFire`
  ;[1 1 1] Fire Weapon System
  (goto _label_2 :!via `Close`))

(event `FirePress`
  (params (Start :type "Vector Structure") (End :type "Vector Structure") (Location :type "Vector Structure"))
  ;[1 1 1] Fire Press and Release
  (set `self.CanFire` true)
  (if (not (`self.IsReloading`))
    (`self.StartFire` Start End Location)))

(event `FireRelease`
  ;[1 1 1] Fire Press and Release
  (set `self.CanFire` false)
  (`self.StopFire`)
  (`self.AutoReload`))

(event `AutoReload`
  ;[1 1 1] Reloading System
  (if (== (`.CurrentAmmo_10_F26B1AC041A51A8482A4EC9820B606C3` (break `/Game/Blueprints/Pickups/ItemType` (`self.ItemInfo`))) 0)
    (if (not (== (`.MaxAmmo_12_5CB6548F43FF84F4CDA05EABE30D38F0` (break `/Game/Blueprints/Pickups/ItemType` (`self.ItemInfo`))) 0))
      (set `self.IsReloading` true)
      (`self.Reloading`)
      (`KismetSystemLibrary.Delay` 2.0)
      (set `self.IsReloading` false))))

(event `Reloading`
  (bind ((`ClipSIze_27_C880D342429160F4E1FB02BDC19C733B` _clipsize) (`CurrentAmmo_10_F26B1AC041A51A8482A4EC9820B606C3` _currentammo)) (break `/Game/Blueprints/Pickups/ItemType` (`self.ItemInfo`)))
  ;[1 1 1] Reloading System
  (if (== (`.MaxAmmo_12_5CB6548F43FF84F4CDA05EABE30D38F0` (break `/Game/Blueprints/Pickups/ItemType` (`self.ItemInfo`))) 0)
    (`KismetSystemLibrary.PrintString` "Find Ammo")
    (elif (== _clipsize _currentammo)
      (`KismetSystemLibrary.PrintString` "Find Ammo")
      (else
        (bind _output_get (set `self.IsReloading` true))
        (if _output_get
          (`self.WeaponReload`)
          (`KismetSystemLibrary.Delay` 2.0)
          (set `self.IsReloading` false))))))

(event `WeaponReload`
  (bind _neededammo (`self.NeededAmmo`))
  (bind _iteminfo (`self.ItemInfo`))
  (bind ((`ClipSIze_27_C880D342429160F4E1FB02BDC19C733B` _clipsize) (`CurrentAmmo_10_F26B1AC041A51A8482A4EC9820B606C3` _currentammo)) (break `/Game/Blueprints/Pickups/ItemType` (`self.ItemInfo`)))
  (bind ((`MaxAmmo_12_5CB6548F43FF84F4CDA05EABE30D38F0` _maxammo)) (break `/Game/Blueprints/Pickups/ItemType` (`self.ItemInfo`)))
  (bind ((`CurrentAmmo_10_F26B1AC041A51A8482A4EC9820B606C3` _currentammo_2) (`MaxAmmo_12_5CB6548F43FF84F4CDA05EABE30D38F0` _maxammo_2)) (break `/Game/Blueprints/Pickups/ItemType` (`self.ItemInfo`)))
  ;[1 1 1] Reloading System
  (if (not (`self.CanFire`))
    (`Character.PlayAnimMontage` (`self.PlayerCharacter`) "/Game/Animations/RifleAnimsetPro/Animations/InPlace/Rifle_Reload_2_Montage.Rifle_Reload_2_Montage" 1.0 "None")
    (if (> (`.MaxAmmo_12_5CB6548F43FF84F4CDA05EABE30D38F0` (break `/Game/Blueprints/Pickups/ItemType` (`self.ItemInfo`))) 0)
      (set `self.NeededAmmo` (- _clipsize _currentammo))
      (if (< _maxammo _neededammo)
        (setmembers `/Game/Blueprints/Pickups/ItemType` :`StructRef` _iteminfo :`CurrentAmmo` (+ _currentammo_2 _maxammo_2))
        (setmembers `/Game/Blueprints/Pickups/ItemType` :`StructRef` _iteminfo :`MaxAmmo` 0)
        (else
          (setmembers `/Game/Blueprints/Pickups/ItemType` :`StructRef` _iteminfo :`MaxAmmo` (- _maxammo _neededammo))
          (setmembers `/Game/Blueprints/Pickups/ItemType` :`StructRef` _iteminfo :`CurrentAmmo` (`.ClipSIze_27_C880D342429160F4E1FB02BDC19C733B` (break `/Game/Blueprints/Pickups/ItemType` (`self.ItemInfo`)))))))))

(fn `On/OffVisibility/CustomDepth`
  (params (bNewVisibility :type Boolean) (bValue :type Boolean))
  (`SceneComponent.SetVisibility` (`self.Widget`) bNewVisibility false)
  (`PrimitiveComponent.SetRenderCustomDepth` (`self.SkeletalMesh`) bValue)
  (return))

(fn `UserConstructionScript`
  (bind (_iteminfo_itemtype _iteminfo_itemclass _iteminfo_clipsize _iteminfo_currentammo _iteminfo_maxammo _iteminfo_damage _iteminfo_itemimage _iteminfo_equipsocketname _iteminfo_unequipsocketname) (break `/Game/Blueprints/Pickups/ItemType` (`self.ItemInfo`)))
  (set `self.ItemInfo` (make `/Game/Blueprints/Pickups/ItemType` _iteminfo_itemtype (`GameplayStatics.GetObjectClass` self) _iteminfo_clipsize _iteminfo_currentammo _iteminfo_maxammo _iteminfo_damage _iteminfo_itemimage _iteminfo_equipsocketname _iteminfo_unequipsocketname)))