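; Sniper ammo pickup that refills the player's sniper when the ItemInteraction input is pressed and a sniper exists.
; It prints a full-ammo message when the weapon's MaxAmmo equals PickupAmmo.
; Otherwise it writes MaxAmmo in the sniper's ItemInfo struct, capped at PickupAmmo, then plays a sound and destroys itself.
; The cap check passes for any non-negative MaxAmmo, so the result is effectively PickupAmmo.
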(event `InputAction|ItemInteraction`
  (params (Key :type "Key Structure" :default "AnyKey"))
  (bind _sniperbp (`/Game/Blueprints/Characters/0_Base.SniperBP` (`self.PlayerCharacter`)))
  (bind _iteminfo (`/Game/Blueprints/Pickups/MasterPickupBP.ItemInfo` (`/Game/Blueprints/Characters/0_Base.SniperBP` (`self.PlayerCharacter`))))
  (bind ((`MaxAmmo_12_5CB6548F43FF84F4CDA05EABE30D38F0` _maxammo)) (break `/Game/Blueprints/Pickups/ItemType` (`/Game/Blueprints/Pickups/MasterPickupBP.ItemInfo` _sniperbp)))
  (bind _returnvalue (+ (`self.PickupAmmo`) _maxammo))
  (:`Pressed`
    (if (`KismetSystemLibrary.IsValid` _sniperbp)
      (if (== _maxammo (`self.PickupAmmo`))
        (`KismetSystemLibrary.PrintString` "Full of Ammo")
        (else
          (if (>= _returnvalue (`self.PickupAmmo`))
            (setmembers `/Game/Blueprints/Pickups/ItemType` :`StructRef` _iteminfo :`MaxAmmo` (`self.PickupAmmo`))
            (else
              (setmembers `/Game/Blueprints/Pickups/ItemType` :`StructRef` _iteminfo :`MaxAmmo` _returnvalue)))
          (`GameplayStatics.PlaySound2D` "/Game/StarterContent/Audio/Collapse_Cue.Collapse_Cue")
          (`self.K2_DestroyActor`))))))

(fn `UserConstructionScript`
  (`parent.UserConstructionScript`))