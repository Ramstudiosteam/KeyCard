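; Rifle ammo pickup that gives ammo to the player when ItemInteraction is pressed.
; The press calls ServerAmmoPickup, then branches on authority to RifleAmmoPickup or inline logic, so PlayerCharacter.RilfleAmmoServer is called twice per press.
; Each call is followed by the PickupCondition macro, which compares a valid rifle's MaxAmmo to PickupAmmo and plays a collapse sound when they differ.
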(event `InputAction|ItemInteraction`
  (params (Key :type "Key Structure" :default "AnyKey"))
  (:`Pressed`
    (`self.ServerAmmoPickup` self)
    (if (`self.HasAuthority`)
      (`self.RifleAmmoPickup` self)
      (else
        (`/Game/Blueprints/Characters/0_Base.RilfleAmmoServer` (`self.PlayerCharacter`) (`self.PickupAmmo`))
        (`self.PickupCondition`
          (:`false`
            (`GameplayStatics.PlaySound2D` "/Game/StarterContent/Audio/Collapse_Cue.Collapse_Cue")))))))

(event `ServerAmmoPickup`
  (params (Target :type "Actor Object Reference"))
  (`/Game/Blueprints/Characters/0_Base.RilfleAmmoServer` (`self.PlayerCharacter`) (`self.PickupAmmo`))
  (`self.PickupCondition`
    (:`false`
      (`GameplayStatics.PlaySound2D` "/Game/StarterContent/Audio/Collapse_Cue.Collapse_Cue"))))

(event `RifleAmmoPickup`
  (params (Target :type "Actor Object Reference"))
  (`/Game/Blueprints/Characters/0_Base.RilfleAmmoServer` (`self.PlayerCharacter`) (`self.PickupAmmo`))
  (`self.PickupCondition`
    (:`false`
      (`GameplayStatics.PlaySound2D` "/Game/StarterContent/Audio/Collapse_Cue.Collapse_Cue"))))

(fn `UserConstructionScript`
  (`parent.UserConstructionScript`))